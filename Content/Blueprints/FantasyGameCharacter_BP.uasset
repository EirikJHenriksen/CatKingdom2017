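; FantasyGameCharacter_BP is the player character Blueprint that handles pausing and triggers the game over and win screens.
; PauseFunction toggles game pause, creating or removing TheMenu widget and showing or hiding the mouse cursor.
; The PauseUnpause input calls it and clears the game instance's MainMenuIsNotActive flag.
; Tick calls the same function when the player is dead or the game instance reports a win.
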(event `InputAction|PauseUnpause` :paused true
  (params (Key :type "Key Structure" :default "AnyKey"))
  ;[1 1 1] Function is also called when pressing "resume" button in pause menu
  (:`Pressed`
    (`self.PauseFunction`)
    (bind _asfantasy_game_instance (cast `FantasyGameInstance` (`GameplayStatics.GetGameInstance`)))
    (set `FantasyGameInstance.MainMenuIsNotActive` false _asfantasy_game_instance)))

(event `self.ReceiveTick`
  (params (DeltaSeconds :type "Float (single-precision)"))
  ;[1 1 1] Makes the game over screen appear when player dies
  (bind _asfantasy_game_character_bp (cast `/Game/Blueprints/FantasyGameCharacter_BP` (`GameplayStatics.GetPlayerCharacter` 0)))
  (if (`Gruppe7_FantasyGameCharacter.PlayerIsDead` _asfantasy_game_character_bp)
    (`self.PauseFunction`)
    (else
      ;[1 1 1] Makes the win screen appear when the game is won
      (bind _asfantasy_game_instance (cast `FantasyGameInstance` (`GameplayStatics.GetGameInstance`)))
      (if (`FantasyGameInstance.GameIsWon` _asfantasy_game_instance)
        (`self.PauseFunction`)))))

(fn `PauseFunction`
  ;[1 1 1] Pause / Unpause
  (cast `Gruppe7_FantasyGameGameMode` (`GameplayStatics.GetGameMode`))
  (`GameplayStatics.SetGamePaused` (not (`GameplayStatics.IsGamePaused`)))
  (if (`GameplayStatics.IsGamePaused`)
    ;[1 1 1] If pausing: bring up a pause menu and mouse curser
    (bind _returnvalue (`|CreateWidget` "/Game/UI/TheMenu.TheMenu_C" (`GameplayStatics.GetPlayerController` 0)))
    (`UserWidget.AddToViewport` _returnvalue 0)
    (set `PlayerController.bShowMouseCursor` true (`GameplayStatics.GetPlayerController` 0))
    (else
      ;[1 1 1] If unpausing: remove pause menu and hide mouse cursor
      (bind _foundwidgets (`WidgetBlueprintLibrary.GetAllWidgetsOfClass` "/Game/UI/TheMenu.TheMenu_C"))
      (`Widget.RemoveFromParent` (`KismetArrayLibrary.Array_Get` _foundwidgets))
      (set `PlayerController.bShowMouseCursor` false (`GameplayStatics.GetPlayerController` 0)))))

(fn `UserConstructionScript`)