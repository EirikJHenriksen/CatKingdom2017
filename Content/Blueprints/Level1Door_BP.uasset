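; Level 1 door that opens automatically when the player holds enough pickups to pay its price and comes within a fixed range.
; Tick checks the character's pickup count and distance, deducts the price, and writes the next door's cost to the game instance for the HUD.
; It then plays a sound, destroys itself and spawns a teleport particle effect.
; An attached evil audio component restarts whenever it finishes, looping continuously.
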(event `self.ReceiveTick`
  (params (DeltaSeconds :type "Float (single-precision)"))
  ;[1 1 1] Check if you have enough pickups for the door
  (bind _asfantasy_game_character_bp (cast `/Game/Blueprints/FantasyGameCharacter_BP` (`GameplayStatics.GetPlayerCharacter` 0)))
  (if (>= (`Gruppe7_FantasyGameCharacter.CollectionPickup` _asfantasy_game_character_bp) (`self.DoorPrice`))
    ;[1 1 1] Then check if you are close enough to door
    (bind _asfantasy_game_character_bp_2 (cast `/Game/Blueprints/FantasyGameCharacter_BP` (`GameplayStatics.GetPlayerCharacter` 0)))
    ;[1 1 1] Remove pickups for opening door
    (if (> 350.0 (`KismetMathLibrary.VSize` (- (`self.K2_GetActorLocation`) (`self.K2_GetActorLocation` _asfantasy_game_character_bp_2))))
      (bind _asfantasy_game_character_bp_3 (cast `/Game/Blueprints/FantasyGameCharacter_BP` (`GameplayStatics.GetPlayerCharacter` 0)))
      (set `Gruppe7_FantasyGameCharacter.CollectionPickup` (- (`Gruppe7_FantasyGameCharacter.CollectionPickup` _asfantasy_game_character_bp_3) (`self.DoorPrice`)) _asfantasy_game_character_bp_3)
      ;[1 1 1] set the price for next door, for displaying in HUD
      (bind _asfantasy_game_instance (cast `FantasyGameInstance` (`GameplayStatics.GetGameInstance`)))
      (set `FantasyGameInstance.NextCost` (`self.NextDoorsPrice`) _asfantasy_game_instance)
      (`GameplayStatics.PlaySoundAtLocation` "/Game/Audio/PlayerSFX/Fire01.Fire01" (`self.K2_GetActorLocation`) (struct) 1.0 1.0 0.0 "/Game/Audio/StandardAttenuation.StandardAttenuation")
      (`self.K2_DestroyActor`)
      (`GameplayStatics.SpawnEmitterAtLocation` "/Game/Particles/P_NightNightTeleport.P_NightNightTeleport" (`self.K2_GetActorLocation`)))))

(event `self.EvilAudio.OnAudioFinished`
  ;[1 1 1] Loops the audio
  (`AudioComponent.Play` (`self.EvilAudio`) 0.0))

(fn `UserConstructionScript`)