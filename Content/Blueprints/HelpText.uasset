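; HelpText is an actor that shows world-space help text, fading it in while the player character is inside its box and out otherwise.
; Each Tick polls the Box overlap and nudges an alpha variable up toward a low cap or down toward zero at twice the rate.
; That alpha is applied to a white TextRender color every frame, with fixed steps that make the fade frame-rate dependent.
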(event `self.ReceiveTick`
  (params (DeltaSeconds :type "Float (single-precision)"))
  (if (`PrimitiveComponent.IsOverlappingActor` (`self.Box`) (`GameplayStatics.GetPlayerCharacter` 0))
    (if (<= (`self.MyAlpha`) 0.255)
      (set `self.MyAlpha` (+ (`self.MyAlpha`) 0.005)))
    (elif (>= (`self.MyAlpha`) 0.0)
      (set `self.MyAlpha` (- (`self.MyAlpha`) 0.01))))
  (`TextRenderComponent.SetTextRenderColor` (`self.TextRender`) (`KismetMathLibrary.Conv_LinearColorToColor` (`KismetMathLibrary.MakeColor` 255.0 255.0 255.0 (`self.MyAlpha`)))))

(fn `UserConstructionScript`)