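; FinalLevelMusic_BP is an actor that handles music for the final level, switching from normal music to fight music during a boss fight.
; Each tick it reads BossFightActive from FantasyGameInstance and, when true, activates the FightMusic audio component and stops NormalMusic.
; Both audio components loop by calling Play again when they finish, and nothing switches back to normal music.
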(event `self.ReceiveTick`
  (params (DeltaSeconds :type "Float (single-precision)"))
  (bind _asfantasy_game_instance (cast `FantasyGameInstance` (`GameplayStatics.GetGameInstance`)))
  (if (`FantasyGameInstance.BossFightActive` _asfantasy_game_instance)
    (`ActorComponent.Activate` (`self.FightMusic`) false)
    (`AudioComponent.Stop` (`self.NormalMusic`))))

(event `self.NormalMusic.OnAudioFinished`
  (`AudioComponent.Play` (`self.NormalMusic`) 0.0))

(event `self.FightMusic.OnAudioFinished`
  (`AudioComponent.Play` (`self.FightMusic`) 0.0))

(fn `UserConstructionScript`)