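; Secret_BP is a breakable actor that is destroyed after enough physical attack hits, likely concealing a secret.
; Its Box overlap counts only PhysAttackBox_BP contacts, playing a hit sound and incrementing a hit counter on each.
; When hits reach Health, it spawns an earth particle effect at its location and destroys itself.
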(event `self.Box.OnComponentBeginOverlap`
  (params (OverlappedComponent :type "PrimitiveComponent Object Reference") (OtherActor :type "Actor Object Reference") (OtherComp :type "PrimitiveComponent Object Reference") (OtherBodyIndex :type Integer) (bFromSweep :type Boolean) (SweepResult :type "HitResult Structure (by ref)"))
  ;[1 1 1] Destroys the actor when it has sustained enough hits
  (cast `/Game/Blueprints/PhysAttackBox_BP` OtherActor)
  (`GameplayStatics.PlaySoundAtLocation` "/Game/Audio/PlayerSFX/Hit01.Hit01")
  (bind _result (`/Engine/EditorBlueprintResources/StandardMacros.IncrementInt` (`self.HitValue`))
    (:`  `
      (set `self.Hits` _result)
      (if (>= (`self.Hits`) (`self.Health`))
        (`GameplayStatics.SpawnEmitterAtLocation` "/Game/Particles/P_ThorneEarth.P_ThorneEarth" (`self.K2_GetActorLocation`))
        (`self.K2_DestroyActor`)))))

(fn `UserConstructionScript`)